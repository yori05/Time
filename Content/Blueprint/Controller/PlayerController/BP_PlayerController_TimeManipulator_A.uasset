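; Player controller that lets the player switch time manipulation between rewinding and recording through Enhanced Input.
; The time-backward action starts the replay state and the time-forward action starts the record state when each input begins.
; Both handlers find the Manager_TMComponent_Basic component on the game mode and call it only if valid, leaving the time logic to that manager.
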(event `EnhancedInput|/Game/Input/Actions/TM_Actions/IA_TimeBackward`
  (params (ActionValue :type Boolean) (ElapsedSeconds :type "Float (double-precision)") (TriggeredSeconds :type "Float (double-precision)") (InputAction :type "InputAction Object Reference" :default "/Game/Input/Actions/TM_Actions/IA_TimeBackward.IA_TimeBackward"))
  (bind _returnvalue (`self.GetComponentByClass` (`GameplayStatics.GetGameMode`) "/Script/Time.Manager_TMComponent_Basic"))
  (:`Started`
    (`/Engine/EditorBlueprintResources/StandardMacros.IsValid` _returnvalue
      (:`Is Valid`
        (`Manager_TMComponent_Basic.LaunchReplayState` _returnvalue)))))

(event `EnhancedInput|/Game/Input/Actions/TM_Actions/IA_TimeForward`
  (params (ActionValue :type Boolean) (ElapsedSeconds :type "Float (double-precision)") (TriggeredSeconds :type "Float (double-precision)") (InputAction :type "InputAction Object Reference" :default "/Game/Input/Actions/TM_Actions/IA_TimeForward.IA_TimeForward"))
  (bind _returnvalue (`self.GetComponentByClass` (`GameplayStatics.GetGameMode`) "/Script/Time.Manager_TMComponent_Basic"))
  (:`Started`
    (`/Engine/EditorBlueprintResources/StandardMacros.IsValid` _returnvalue
      (:`Is Valid`
        (`Manager_TMComponent_Basic.LaunchRecordState` _returnvalue)))))

(fn `UserConstructionScript`
  (`parent.UserConstructionScript`))